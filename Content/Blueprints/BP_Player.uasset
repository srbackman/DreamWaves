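; Player Blueprint for a click-driven music mixer, where reactive balls switch between two sets of audio tracks and their layers.
; BeginPlay shows the cursor, adds the input mapping and mutes all tracks; clicks are matched to the Balls array by cursor trace.
; The first two balls pick the set and solo its base track; the rest act as either/or pairs, crossfading tracks at set-dependent index offsets.
; Tracks switch only through AdjustVolume fades, never stop/start.
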(event Input|EnhancedActionEvents|EnhancedInputActionIA_Click
  (params (ActionValue :type Boolean) (ElapsedSeconds :type Float%20%28double-precision%29) (TriggeredSeconds :type Float%20%28double-precision%29) (InputAction :type Input%20Action%20Object%20Reference :default "/Game/Input/IA_Click.IA_Click"))
  (bind _balls (Variables|Default|GetBalls))
  (:Triggered
    (bind _asplayer_controller (Utilities|Casting|CastToPlayerController (Pawn|GetController)))
    ;[1 1 1] CanClickOnlyBalls
    (bind _array_element (Utilities|Array|ForEachLoopwithBreak _balls :!label _label)
      (:LoopBody
        (if (== _array_element (.HitActor (Collision|BreakHitResult (.HitResult (Game|Player|GetHitResultUnderCursorbyChannel _asplayer_controller "TraceTypeQuery1" true)))))
          (Variables|Default|SetValidBall true)
          (goto _label Break)))
      (:Completed
        (if (Variables|Default|GetValidBall)
          (if (or (== (.HitActor (Collision|BreakHitResult (.HitResult (Game|Player|GetHitResultUnderCursorbyChannel _asplayer_controller "TraceTypeQuery1" true)))) (Utilities|Array|Get(acopy) _balls)) (== (.HitActor (Collision|BreakHitResult (.HitResult (Game|Player|GetHitResultUnderCursorbyChannel _asplayer_controller "TraceTypeQuery1" true)))) (Utilities|Array|Get(acopy) _balls 1)))
            ;[1 1 1] Balls
            (CallFunction|ResetBalls (.HitActor (Collision|BreakHitResult (.HitResult (Game|Player|GetHitResultUnderCursorbyChannel _asplayer_controller "TraceTypeQuery1" true)))))
            (else
              (bind (_onindex _offindex) (CallFunction|PairControll (.HitActor (Collision|BreakHitResult (.HitResult (Game|Player|GetHitResultUnderCursorbyChannel _asplayer_controller "TraceTypeQuery1" true)))) _balls))
              ;[1 1 1] Music
              (CallFunction|AudioSwitcher _onindex _offindex (Variables|Default|GetMusicSwitchTime)))))))))

(event Input|EnhancedActionEvents|EnhancedInputActionIA_Quit
  (params (ActionValue :type Boolean) (ElapsedSeconds :type Float%20%28double-precision%29) (TriggeredSeconds :type Float%20%28double-precision%29) (InputAction :type Input%20Action%20Object%20Reference :default "/Game/Input/IA_Quit.IA_Quit"))
  (:Triggered
    (Game|QuitGame 0 "Quit" false)))

(event EventBeginPlay
  (bind _returnvalue (Game|GetPlayerController 0))
  (Utilities|FlowControl|Sequence
    (:then_0
      ;[1 1 1] Comment
      (Variables|/Script/Engine.PlayerController|SetbShowMouseCursor _returnvalue true)
      (Input|SetIgnoreMoveInput _returnvalue false))
    (:then_1
      ;[1 1 1] Comment
      (bind _asplayer_controller (Utilities|Casting|CastToPlayerController (Pawn|GetController)))
      (Input|AddMappingContext (PlayerController|LocalPlayerSubsystems|GetEnhancedInputLocalPlayerSubsystem _asplayer_controller) (Variables|Default|GetInputMapping) 0 "(bIgnoreAllPressedKeysUntilRelease=True,bForceImmediately=False)"))
    (:then_2
      (CallFunction|MuteEverything))))

(event Collision|EventActorBeginOverlap
  (params (OtherActor :type Actor%20Object%20Reference)))

(event EventTick
  (params (DeltaSeconds :type Float%20%28single-precision%29)))

(fn ConstructionScript)

(fn ResetBalls
  (params (NewParam :type Actor%20Object%20Reference))
  (for (_array_element _array_index) (Variables|Default|GetBalls)
    (if (== NewParam _array_element)
      (bind _asbp_reactive_ball (Utilities|Casting|CastToBP_ReactiveBall _array_element))
      (Default|SetActive _asbp_reactive_ball true)
      (if (== _array_index 0)
        (CallFunction|MuteEverythingButOne _array_index)
        (Variables|Default|SetMusicCurrent 0)
        (else
          (CallFunction|MuteEverythingButOne (+ _array_index 6))
          (Variables|Default|SetMusicCurrent 1)))
      (else
        (bind _asbp_reactive_ball_2 (Utilities|Casting|CastToBP_ReactiveBall _array_element))
        (Default|SetActive _asbp_reactive_ball_2 false)))))

(fn PairControll
  (params (TargetBall :type Actor%20Object%20Reference) (TargetBalls :type Array%20of%20Actor%20Object%20References))
  ;[1 1 1] ManageActiveColors
  (bind _asbp_reactive_ball (Utilities|Casting|CastToBP_ReactiveBall TargetBall))
  (Default|SetActive _asbp_reactive_ball true)
  (bind (_array_element _array_index) (Utilities|Array|ForEachLoopwithBreak TargetBalls)
    (:LoopBody
      ;;[1 1 1] WhileNotStartingBalls
      (if (> _array_index 1)
        (if (== TargetBall _array_element)
          (LocalVariables|SetIndex1 _array_index)
          (if (== (Math|Integer|%(Integer) _array_index 2) 0)
            (LocalVariables|SetIndex2 (+ _array_index 1))
            (bind _asbp_reactive_ball_2 (Utilities|Casting|CastToBP_ReactiveBall (Utilities|Array|Get(acopy) TargetBalls (+ _array_index 1))))
            (Default|SetActive _asbp_reactive_ball_2 false)
            (return (LocalVariables|GetIndex1) (LocalVariables|GetIndex2))
            (else
              (LocalVariables|SetIndex2 (- _array_index 1))
              (bind _asbp_reactive_ball_3 (Utilities|Casting|CastToBP_ReactiveBall (Utilities|Array|Get(acopy) TargetBalls (- _array_index 1))))
              (Default|SetActive _asbp_reactive_ball_3 false)
              (return (LocalVariables|GetIndex1) (LocalVariables|GetIndex2)))))))))

(fn MuteEverything
  ;[1 1 1] MuteEverything
  (for _array_element (Variables|Default|GetTracks)
    (Audio|Components|Audio|AdjustVolume (Actor|GetComponentbyClass _array_element "/Script/Engine.AudioComponent") 0.0 0.001 "Linear" :!class /Script/Engine.AudioComponent)))

(fn MuteEverythingButOne
  (params (Index :type Integer))
  (bind _musicswitchtime (Variables|Default|GetMusicSwitchTime))
  (for (_array_element _array_index) (Variables|Default|GetTracks)
    (if (!= _array_index Index)
      (Audio|Components|Audio|AdjustVolume (Actor|GetComponentbyClass _array_element "/Script/Engine.AudioComponent") _musicswitchtime 0.001 "Linear" :!class /Script/Engine.AudioComponent)
      (Development|PrintString (Utilities|GetDisplayName (Actor|GetComponentbyClass _array_element "/Script/Engine.AudioComponent")) true true "(R=1.000000,G=0.057610,B=0.000000,A=1.000000)")
      (else
        (Audio|Components|Audio|AdjustVolume (Actor|GetComponentbyClass _array_element "/Script/Engine.AudioComponent") _musicswitchtime (Variables|Default|GetMusicVolume) "Linear" :!class /Script/Engine.AudioComponent)
        (Development|PrintString (Utilities|GetDisplayName (Actor|GetComponentbyClass _array_element "/Script/Engine.AudioComponent")) true true "(R=0.228102,G=1.000000,B=0.000000,A=1.000000)")))))

(fn AudioSwitcher
  (params (OnIndex :type Integer) (OffIndex :type Integer) (SwitchTime :type Float%20%28double-precision%29))
  (bind _tracks (Variables|Default|GetTracks))
  (if (== (Variables|Default|GetMusicCurrent) 0)
    (LocalVariables|SetTemp -1)
    (else
      (LocalVariables|SetTemp 6)))
  (Audio|Components|Audio|AdjustVolume (Actor|GetComponentbyClass (Utilities|Array|Get(acopy) _tracks (+ OnIndex (LocalVariables|GetTemp))) "/Script/Engine.AudioComponent") SwitchTime (Variables|Default|GetMusicVolume) "Linear" :!class /Script/Engine.AudioComponent)
  (Audio|Components|Audio|AdjustVolume (Actor|GetComponentbyClass (Utilities|Array|Get(acopy) _tracks (+ OffIndex (LocalVariables|GetTemp))) "/Script/Engine.AudioComponent") SwitchTime 0.001 "Linear" :!class /Script/Engine.AudioComponent)
  (Development|PrintString (Utilities|String|ToString(Boolean) (Audio|Components|Audio|IsPlaying (Actor|GetComponentbyClass (Utilities|Array|Get(acopy) _tracks (+ OnIndex (LocalVariables|GetTemp))) "/Script/Engine.AudioComponent")))))