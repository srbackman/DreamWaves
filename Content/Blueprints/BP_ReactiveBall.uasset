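; Reactive ball actor whose sphere material switches between configurable on and off looks.
; The construction script creates a dynamic material instance on the sphere and applies the off look.
; SetActive picks the on or off color, emission, metallic and roughness values and passes them to ChangeMaterial, which writes the material parameters.
; Clicking the sphere only prints a debug string, and nothing in this Blueprint calls SetActive.
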(event OnClicked(Sphere)
  (params (TouchedComponent :type Primitive%20Component%20Object%20Reference) (ButtonPressed :type Key%20Structure))
  (Development|PrintString "Hello"))

(event EventBeginPlay)

(event Collision|EventActorBeginOverlap
  (params (OtherActor :type Actor%20Object%20Reference)))

(event EventTick
  (params (DeltaSeconds :type Float%20%28single-precision%29)))

(fn ConstructionScript
  (Utilities|FlowControl|Sequence
    (:then_0
      ;[1 1 1] GetMaterial
      (bind _returnvalue (Rendering|Material|CreateDynamicMaterialInstance (Variables|Default|GetSphere) 0 0 "None" :!class /Script/Engine.PrimitiveComponent))
      (Variables|Default|SetCollection _returnvalue))
    (:then_1
      (CallFunction|ChangeMaterial (Variables|Default|GetOffColor) (Variables|Default|GetOffEmissionStrength) (Variables|Default|GetOffMetallic) (Variables|Default|GetOffRoughness)))))

(fn ChangeMaterial
  (params (NewColor :type Color%20Structure) (NewEmissionStrength :type Float%20%28double-precision%29) (NewMetallic :type Float%20%28double-precision%29) (NewRoughness :type Float%20%28double-precision%29))
  (bind _collection (Variables|Default|GetCollection))
  ;[1 1 1] SetMaterialColor
  (if (Utilities|IsValid _collection)
    (Rendering|Material|SetVectorParameterValue _collection "Color" (Math|Conversions|ToLinearColor(Color) NewColor) :!class /Script/Engine.MaterialInstanceDynamic)
    ;[1 1 1] SetMaterialEmissionStrength
    (Rendering|Material|SetScalarParameterValue _collection "EmissionStrength" NewEmissionStrength :!class /Script/Engine.MaterialInstanceDynamic)
    ;[1 1 1] SetMaterialMetallic
    (Rendering|Material|SetScalarParameterValue _collection "Metallic" NewMetallic :!class /Script/Engine.MaterialInstanceDynamic)
    ;[1 1 1] SetMaterialRoughness
    (Rendering|Material|SetScalarParameterValue _collection "Roughness" NewRoughness :!class /Script/Engine.MaterialInstanceDynamic)))

(fn SetActive
  (params (State :type Boolean))
  (if State
    (CallFunction|ChangeMaterial (Variables|Default|GetOnColor) (Variables|Default|GetOnEmissionStrength) (Variables|Default|GetOnMetallic) (Variables|Default|GetOnRoughness))
    (else
      (CallFunction|ChangeMaterial (Variables|Default|GetOffColor) (Variables|Default|GetOffEmissionStrength) (Variables|Default|GetOffMetallic) (Variables|Default|GetOffRoughness)))))